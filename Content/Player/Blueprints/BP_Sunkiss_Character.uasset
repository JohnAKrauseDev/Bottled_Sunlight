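; Player character Blueprint for Sunkiss, with camera-relative movement, a carried light level and interaction with registered objects.
; A looping timer activates the closest registered interactable, which receives primary and secondary interact input.
; AlterLightLevel changes the level by step, preset fraction or override against an expandable maximum, resizing the point light's radius.
; At zero light, a timeline-faded NightLight turns on; debug keys adjust the level and toggle that light.
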(event `self.ReceiveBeginPlay`
  (bind _returnvalue (`KismetSystemLibrary.K2_SetTimer` null "CalculateActiveInteractable" 0.3 true))
  (set `self.CalcInteractableTimer` _returnvalue))

(event `EnhancedInput|/Game/Player/Inputs/IA_Move`
  (params (ActionValue :type "Vector2D Structure") (ElapsedSeconds :type "Float (double-precision)") (TriggeredSeconds :type "Float (double-precision)") (InputAction :type "InputAction Object Reference" :default "/Game/Player/Inputs/IA_Move.IA_Move"))
  ;[1 1 1] Moving
  (:`Triggered`
    (`self.Walking`)))

(event `EnhancedInput|/Game/Player/Inputs/IA_Interact`
  (params (ActionValue :type Boolean) (ElapsedSeconds :type "Float (double-precision)") (TriggeredSeconds :type "Float (double-precision)") (InputAction :type "InputAction Object Reference" :default "/Game/Player/Inputs/IA_Interact.IA_Interact"))
  (bind _activeinteractableref (`self.ActiveInteractableRef`))
  (:`Triggered`
    (`/Engine/EditorBlueprintResources/StandardMacros.IsValid` _activeinteractableref
      (:`Is Valid`
        (`/Game/Props/Blueprints/Interactables/BP_WorldInteractInterface.PrimaryInteract` _activeinteractableref self)))))

(event `EnhancedInput|/Game/Player/Inputs/IA_SecondaryInteract`
  (params (ActionValue :type Boolean) (ElapsedSeconds :type "Float (double-precision)") (TriggeredSeconds :type "Float (double-precision)") (InputAction :type "InputAction Object Reference" :default "/Game/Player/Inputs/IA_SecondaryInteract.IA_SecondaryInteract"))
  (bind _activeinteractableref (`self.ActiveInteractableRef`))
  (:`Triggered`
    (`/Engine/EditorBlueprintResources/StandardMacros.IsValid` _activeinteractableref
      (:`Is Valid`
        (message `/Game/Props/Blueprints/Interactables/BP_WorldInteractInterface.SecondaryInteract` _activeinteractableref self)))))

(event `Key|V`
  (params (Key :type "Key Structure"))
  ;[1 1 1] DevAlterLightLevel
  (:`Pressed`
    (`self.AlterLightLevel` 1)))

(event `Key|C`
  (params (Key :type "Key Structure"))
  ;[1 1 1] DevAlterLightLevel
  (:`Pressed`
    (`self.AlterLightLevel` -1)))

(event `Key|X`
  (params (Key :type "Key Structure"))
  ;[1 1 1] NightLight
  ;;[1 1 1] DevActivateNightLight
  (:`Pressed`
    (`/Engine/EditorBlueprintResources/StandardMacros.FlipFlop`
      (:`A`
        (`SceneComponent.SetVisibility` (`self."NightLight"`) true false :!label _label)
        (bind (_direction __ofbrightness) (`Timeline|NightLightTimeline` :!label _label_2)
          (:`Update`
            (`LightComponent.SetIntensity` (`self."NightLight"`) (`KismetMathLibrary.Lerp` (`self.NightLightMin`) (`self.NightLightMax`) __ofbrightness)))
          (:`Finished`
            (switch `ETimelineDirection` _direction
              (:`Forward`
                (`KismetSystemLibrary.PrintString` "full bright"))
              (:`Backward`
                (`SceneComponent.SetVisibility` (`self."NightLight"`) false false))))))
      (:`B`
        (goto _label_2 :!via `Reverse`)))))

(event `ToggleNightLight`
  (params (TurnOn :type Boolean))
  ;[1 1 1] NightLight
  (if TurnOn
    (goto _label)
    (else
      (goto _label_2 :!via `Reverse`))))

(fn `Add Interactable Ref`
  (params (NewReference :type "/Game/Props/Blueprints/Interactables/BP_InteractableParent Object Reference"))
  (`KismetArrayLibrary.Array_AddUnique` (`self.InteractableRefs`) NewReference))

(fn `AddMaxLight`
  (params (BottleHasLight :type Boolean))
  (`/Engine/EditorBlueprintResources/StandardMacros.IncrementInt` (`self.MaxLightLevel`)
    (:`  `
      (if BottleHasLight
        (`self.AlterLightLevel` 1)))))

(fn `AlterLightLevel`
  (params (`ValueTo"add" +-` :type Integer) (OverwriteLightState :type "/Game/Player/Enums/LightStatesEnum Enum" :default "NewEnumerator0") (OverwriteLightValue :type Boolean) (`NewValue(min 0)` :type Integer))
  (returns (Success :type Boolean))
  (bind _returnvalue (`KismetMathLibrary.Conv_IntToDouble` (`self.MaxLightLevel`)))
  (bind _returnvalue_2 (+ (`self.LightLevel`) `ValueTo"add" +-`))
  (`|ExecutionSequence`
    (:`then_0`
      (if OverwriteLightValue
        (set `self.LightLevel` (`KismetMathLibrary.Max` `NewValue(min 0)`))
        (else
          (switch `/Game/Player/Enums/LightStatesEnum` OverwriteLightState
            (:`NewEnumerator0`
              (if (>= _returnvalue_2 0)
                (if (<= _returnvalue_2 (`self.MaxLightLevel`))
                  (set `self.LightLevel` _returnvalue_2)
                  (else
                    (return false)))
                (else
                  (`KismetSystemLibrary.PrintString` "SunkissedChar Attempted to lower lightLevel; below 0" true true (struct :`R` 1.0 :`G` 0.574654 :`A` 1.0) 10.0)
                  (return false))))
            (:`NewEnumerator1`
              (set `self.LightLevel` (`self.MaxLightLevel`)))
            (:`NewEnumerator2`
              (set `self.LightLevel` (`KismetMathLibrary.FCeil` (* _returnvalue 0.75))))
            (:`NewEnumerator3`
              (set `self.LightLevel` (`KismetMathLibrary.FCeil` (* _returnvalue 0.5))))
            (:`NewEnumerator4`
              (set `self.LightLevel` (`KismetMathLibrary.FCeil` (* _returnvalue 0.25))))
            (:`NewEnumerator5`
              (set `self.LightLevel` 0))))))
    (:`then_1`
      (`self.INTERNAL AdjustBrightness`)
      (return true))))

(fn `CalculateActiveInteractable`
  (locals (CandidateInteractable :type "/Game/Props/Blueprints/Interactables/BP_InteractableParent Object Reference") (CandidateDistance :type "Float (double-precision)"))
  (bind _interactablerefs (`self.InteractableRefs`))
  (bind _activeinteractableref (`self.ActiveInteractableRef`))
  ;[1 1 1] If None, dont bother checking
  (if (`KismetArrayLibrary.Array_IsNotEmpty` (`self.InteractableRefs`))
    ;[1 1 1] If ther is only one, it is active
    (if (> (`KismetArrayLibrary.Array_Length` _interactablerefs) 1)
      ;[1 1 1] If more than one, find closest
      (for (_array_element _array_index) (`self.InteractableRefs`)
        (switch `int` _array_index
          (:`Default`
            (bind _returnvalue (`self.GetDistanceTo` _array_element))
            (if (< _returnvalue (`local.CandidateDistance`))
              (set `local.CandidateInteractable` _array_element)
              (set `local.CandidateDistance` _returnvalue)))
          (:`0`
            (bind _output_get (set `local.CandidateInteractable` _array_element))
            (set `local.CandidateDistance` (`self.GetDistanceTo` _output_get)))))
      ;[1 1 1] Do Nothing if old is still current active
      (if (not (== (`self.ActiveInteractableRef`) (`local.CandidateInteractable`)))
        ;[1 1 1] If new active, change status in relevant actors
        (`/Engine/EditorBlueprintResources/StandardMacros.IsValid` (`self.ActiveInteractableRef`)
          (:`Is Valid`
            (`/Game/Props/Blueprints/Interactables/BP_InteractableParent.EndActive` (`self.ActiveInteractableRef`)))
          (:`Is Not Valid`
            _))
        (bind _output_get_2 (set `self.ActiveInteractableRef` (`local.CandidateInteractable`)))
        (`/Game/Props/Blueprints/Interactables/BP_InteractableParent.BecomeActive` _output_get_2))
      (else
        ;[1 1 1] Do Nothing if old is still current active
        (if (not (== _activeinteractableref (`|GetArrayItem` (`self.InteractableRefs`))))
          ;[1 1 1] EndOld,StartNew
          (`/Engine/EditorBlueprintResources/StandardMacros.IsValid` _activeinteractableref
            (:`Is Valid`
              (`/Game/Props/Blueprints/Interactables/BP_InteractableParent.EndActive` _activeinteractableref))
            (:`Is Not Valid`
              _))
          (bind _output_get_3 (set `self.ActiveInteractableRef` (`|GetArrayItem` _interactablerefs)))
          (`/Game/Props/Blueprints/Interactables/BP_InteractableParent.BecomeActive` _output_get_3))))))

(fn `INTERNAL AdjustBrightness`
  (`LocalLightComponent.SetAttenuationRadius` (`self.PointLight`) (* (`self.RadiusPerLevel`) (`self.LightLevel`)))
  (switch `int` (`self.LightLevel`)
    (:`Default`
      (`self.ToggleNightLight` false))
    (:`0`
      (`self.ToggleNightLight` true))))

(fn `RemoveInteractableRef`
  (params (`Ref To Remove` :type "/Game/Props/Blueprints/Interactables/BP_InteractableParent Object Reference"))
  (bind _activeinteractableref (`self.ActiveInteractableRef`))
  (`KismetArrayLibrary.Array_RemoveItem` (`self.InteractableRefs`) `Ref To Remove`)
  ;[1 1 1] If actor being removed is same as current active, set it not active
  (if (== `Ref To Remove` _activeinteractableref)
    (`/Game/Props/Blueprints/Interactables/BP_InteractableParent.EndActive` _activeinteractableref)
    (set `self.ActiveInteractableRef` null)))

(fn `UserConstructionScript`
  (bind _pointlight (`self.PointLight`))
  (`LightComponent.SetIntensity` _pointlight (* (`self.BrightnessPerLevel`) (`self.LightLevel`)))
  (`LocalLightComponent.SetAttenuationRadius` _pointlight (* (`self.RadiusPerLevel`) (`self.LightLevel`)))
  (`LightComponent.SetIntensity` (`self."NightLight"`) (`self.NightLightMin`)))

(fn `Walking`
  (bind (_returnvalue_x _returnvalue_y) (`KismetMathLibrary.BreakVector2D` (`|GetInputActionValue`)))
  (bind _camera (`self.Camera`))
  (bind (_returnvalue_x_2 _returnvalue_y_2) (`KismetMathLibrary.BreakVector` (`SceneComponent.GetForwardVector` _camera)))
  (bind (_returnvalue_x_3 _returnvalue_y_3) (`KismetMathLibrary.BreakVector` (`SceneComponent.GetRightVector` _camera)))
  (`self.AddMovementInput` (+ (* (`KismetMathLibrary.GetDirectionUnitVector` (0.0 0.0 0.0) (`KismetMathLibrary.MakeVector` _returnvalue_x_2 _returnvalue_y_2)) _returnvalue_x) (* (`KismetMathLibrary.GetDirectionUnitVector` (0.0 0.0 0.0) (`KismetMathLibrary.MakeVector` _returnvalue_x_3 _returnvalue_y_3)) _returnvalue_y))))