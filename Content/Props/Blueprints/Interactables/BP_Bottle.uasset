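; BP_Bottle is an interactable bottle pickup that calls AddMaxLight on the Sunkiss character that uses it.
; PrimaryInteract casts the instigator to BP_Sunkiss_Character, makes that call, starts a short timer and returns false.
; The timer calls Delayed Destroy Self by name, removing the bottle just after the interaction instead of during it.
; The event graph holds only disabled default events.
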(fn `Delayed Destroy Self`
  (`self.K2_DestroyActor`))

(fn `PrimaryInteract`
  (params (Instegator :type "Actor Object Reference"))
  (returns (Success :type Boolean))
  (bind _asbp_sunkiss_character (cast `/Game/Player/Blueprints/BP_Sunkiss_Character` Instegator))
  (`/Game/Player/Blueprints/BP_Sunkiss_Character.AddMaxLight` _asbp_sunkiss_character true)
  (`KismetSystemLibrary.K2_SetTimer` null "Delayed Destroy Self" 0.1)
  (return false))

(fn `UserConstructionScript`
  (`parent.UserConstructionScript`))