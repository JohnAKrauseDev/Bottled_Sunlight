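; Base Blueprint for interactable props, providing an interaction volume and stub functions for children to override.
; Construction sizes and rotates the interaction capsule from per-instance variables.
; When HasInteraction is set, overlaps add or remove the actor as an interactable reference on BP_Sunkiss_Character, with a DoOnce blocking duplicate adds until no character overlaps.
; BecomeActive and EndActive only print debug text, while PrimaryInteract and SecondaryInteract return false.
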(event `self.InteractionCollision.OnComponentBeginOverlap`
  (params (OverlappedComponent :type "PrimitiveComponent Object Reference") (OtherActor :type "Actor Object Reference") (OtherComp :type "PrimitiveComponent Object Reference") (OtherBodyIndex :type Integer) (bFromSweep :type Boolean) (SweepResult :type "HitResult Structure (by ref)"))
  ;[1 1 1] Give/Remove Reference
  (if (`self.HasInteraction`)
    (bind _asbp_sunkiss_character (cast `/Game/Player/Blueprints/BP_Sunkiss_Character` OtherActor))
    (`/Engine/EditorBlueprintResources/StandardMacros.DoOnce` false :!label _label
      (:`Completed`
        (`/Game/Player/Blueprints/BP_Sunkiss_Character.Add Interactable Ref` _asbp_sunkiss_character self)))))

(event `self.InteractionCollision.OnComponentEndOverlap`
  (params (OverlappedComponent :type "PrimitiveComponent Object Reference") (OtherActor :type "Actor Object Reference") (OtherComp :type "PrimitiveComponent Object Reference") (OtherBodyIndex :type Integer))
  ;[1 1 1] Give/Remove Reference
  (if (`self.HasInteraction`)
    (bind _asbp_sunkiss_character (cast `/Game/Player/Blueprints/BP_Sunkiss_Character` OtherActor))
    (if (`KismetArrayLibrary.Array_IsEmpty` (`PrimitiveComponent.GetOverlappingActors` (`self.InteractionCollision`) "/Game/Player/Blueprints/BP_Sunkiss_Character.BP_Sunkiss_Character_C"))
      (`|ExecutionSequence`
        (:`then_0`
          (goto _label :!via `Reset`))
        (:`then_1`
          (`/Game/Player/Blueprints/BP_Sunkiss_Character.RemoveInteractableRef` _asbp_sunkiss_character self))))))

(fn `BecomeActive`
  (`KismetSystemLibrary.PrintString` "Interact parent Set ActiveTrue(usewithtext)"))

(fn `EndActive`
  (`KismetSystemLibrary.PrintString` "Interact parent Set ActiveFalse(usewithtext)"))

(fn `PrimaryInteract`
  (params (Instegator :type "Actor Object Reference"))
  (returns (Success :type Boolean))
  (return false))

(fn `SecondaryInteract`
  (params (Instegator :type "Actor Object Reference"))
  (returns (Success :type Boolean))
  (return false))

(fn `UserConstructionScript`
  (bind _interactioncollision (`self.InteractionCollision`))
  (`|ExecutionSequence`
    (:`then_1`
      ;[1 1 1] CollisionSetup
      (`CapsuleComponent.SetCapsuleRadius` _interactioncollision (`self.Interact Radius`) true)
      (`CapsuleComponent.SetCapsuleHalfHeight` _interactioncollision (`self.Interact Half Height`) true)
      (`SceneComponent.K2_SetRelativeRotation` _interactioncollision (`self.Interact Rotation`) false false))))