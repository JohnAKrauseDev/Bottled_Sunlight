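; BP_Battery is an interactable power prop that stores light transferred from the player and powers linked dependants only while full.
; Primary interact moves one light level from the player into the battery, and secondary interact takes one back.
; The construction script spawns a centred row of child-actor indicator lights, one per capacity unit, which switch on or off with the stored level.
; On BeginPlay it registers itself as a power source on each dependant.
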(event `self.ReceiveBeginPlay`
  (`parent.ReceiveBeginPlay`)
  ;[1 1 1] Give dependants reference to self if dont already have one
  (for _array_element (`self.DependantRefs`)
    (`/Engine/EditorBlueprintResources/StandardMacros.IsValid` _array_element
      (:`Is Valid`
        (bind _powersources (`/Game/Props/Blueprints/Interactables/Powered/BP_PoweredParent.PowerSources` _array_element))
        (if (not (`KismetArrayLibrary.Array_Contains` _powersources self))
          (`KismetArrayLibrary.Array_Add` _powersources self))))))

(event `self.ReceiveTick`
  (params (DeltaSeconds :type "Float (single-precision)"))
  (`parent.ReceiveTick` DeltaSeconds))

(fn `ActivateDependants`
  (set `self.IsOutputingPower` true)
  (for _array_element (`self.DependantRefs`)
    (`/Game/Props/Blueprints/Interactables/Powered/BP_PoweredParent.StartRecievePower` _array_element)))

(fn `AlterStoredLight`
  (params (`Amount to add +-` :type Integer))
  (returns (Success :type Boolean))
  (bind _returnvalue (+ `Amount to add +-` (`self.StoredLightLevel`)))
  (`|ExecutionSequence`
    (:`then_0`
      (if (and (>= _returnvalue 0) (<= _returnvalue (`self.Capacity`)))
        (bind _output_get (set `self.StoredLightLevel` _returnvalue))
        (if (== _output_get (`self.Capacity`))
          (`self.ActivateDependants`)
          (elif (`self.IsOutputingPower`)
            (`self.DeactivateDependants`)))
        (else
          (return false))))
    (:`then_1`
      (`self.INTERNAL AdjustBateryLights`))))

(fn `DeactivateDependants`
  (set `self.IsOutputingPower` false)
  (for _array_element (`self.DependantRefs`)
    (`/Game/Props/Blueprints/Interactables/Powered/BP_PoweredParent.EndRecievePower` _array_element)))

(fn `INTERNAL AdjustBateryLights`
  (for (_array_element _array_index) (`self.BatteryLightRefs`)
    (if (<= _array_index (- (`self.StoredLightLevel`) 1))
      (`/Game/Props/Blueprints/Interactables/Battery/BP_BatteryLightComponent.TurnOn` _array_element)
      (else
        (`/Game/Props/Blueprints/Interactables/Battery/BP_BatteryLightComponent.TurnOff` _array_element)))))

(fn `PrimaryInteract`
  (params (Instegator :type "Actor Object Reference"))
  (returns (Success :type Boolean))
  (bind _asbp_sunkiss_character (cast `/Game/Player/Blueprints/BP_Sunkiss_Character` Instegator)
    (:`then`
      ;[1 1 1] Do nothing if at capacity
      (if (>= (`self.StoredLightLevel`) (`self.Capacity`))
        (return false)
        (else
          ;[1 1 1] check if light above 1
          (if (> (`/Game/Player/Blueprints/BP_Sunkiss_Character.LightLevel` _asbp_sunkiss_character) 1)
            ;[1 1 1] Success
            (`self.AlterStoredLight` 1)
            (`/Game/Player/Blueprints/BP_Sunkiss_Character.AlterLightLevel` _asbp_sunkiss_character -1 "NewEnumerator0" false 0)
            (return true)
            (else
              ;[1 1 1] Check if at 1
              (if (== (`/Game/Player/Blueprints/BP_Sunkiss_Character.LightLevel` _asbp_sunkiss_character) 1)
                ;[1 1 1] Special behavior for last light level? set this in player?
                (`KismetSystemLibrary.PrintString` "add special behavior for last light level to be givren?")
                (`self.AlterStoredLight` 1)
                (`/Game/Player/Blueprints/BP_Sunkiss_Character.AlterLightLevel` _asbp_sunkiss_character -1 "NewEnumerator0" false 0)
                (return true)
                (else
                  (return false))))))))
    (:`CastFailed`
      (`KismetSystemLibrary.PrintString` "Battery make interaction with non player")
      (return false))))

(fn `SecondaryInteract`
  (params (Instegator :type "Actor Object Reference"))
  (returns (Success :type Boolean))
  (bind _asbp_sunkiss_character (cast `/Game/Player/Blueprints/BP_Sunkiss_Character` Instegator)
    (:`then`
      ;[1 1 1] Fail if at player at max light
      (if (>= (`/Game/Player/Blueprints/BP_Sunkiss_Character.LightLevel` _asbp_sunkiss_character) (`/Game/Player/Blueprints/BP_Sunkiss_Character.MaxLightLevel` _asbp_sunkiss_character))
        (return false)
        (else
          ;[1 1 1] Do nothing if empty
          (if (<= (`self.StoredLightLevel`) 0)
            (return false)
            (else
              ;[1 1 1] Success
              (`self.AlterStoredLight` -1)
              (`/Game/Player/Blueprints/BP_Sunkiss_Character.AlterLightLevel` _asbp_sunkiss_character 1 "NewEnumerator0" false 0)
              (return true))))))
    (:`CastFailed`
      (`KismetSystemLibrary.PrintString` "Battery make Secondary interaction with non player")
      (return false))))

(fn `UserConstructionScript`
  (locals (invalidRefs :type Boolean))
  (bind _batterylightscale (`self.BatteryLightScale`))
  (bind _returnvalue (- (`self.Capacity`) 1))
  (`parent.UserConstructionScript`)
  (for _index (range (+ _returnvalue 1))
    (bind _returnvalue_2 (`AddComponent|NODE_AddChildActorComponent-0` :`RelativeTransform` (`KismetMathLibrary.MakeTransform` (+ (`SceneComponent.RelativeLocation` (`self.BatteryLightCenter`)) (* (`self.BalleryLightOffset`) _index)))))
    (`ChildActorComponent.SetChildActorClass` _returnvalue_2 "/Game/Props/Blueprints/Interactables/Battery/BP_BatteryLightComponent.BP_BatteryLightComponent_C")
    (bind (_success _ref) (message `/Game/Props/Blueprints/Interactables/ChildReferenceInterface.GetBatteryLightRef` (`ChildActorComponent.ChildActor` _returnvalue_2)))
    (if _success
      (`KismetArrayLibrary.Array_Add` (`self.BatteryLightRefs`) _ref)
      (else
        (`KismetSystemLibrary.PrintString` "BP_Battery: Construction script child reference failed"))))
  (for _array_element (`self.BatteryLightRefs`)
    (`/Engine/EditorBlueprintResources/StandardMacros.IsValid` _array_element
      (:`Is Valid`
        (bind _batterymesh (`/Game/Props/Blueprints/Interactables/Battery/BP_BatteryLightComponent.BatteryMesh` _array_element))
        (`SceneComponent.SetRelativeScale3D` _batterymesh (`KismetMathLibrary.MakeVector` _batterylightscale _batterylightscale _batterylightscale))
        (`StaticMeshComponent.SetStaticMesh` _batterymesh (`self.BatteryLightMesh`))
        (`SceneComponent.K2_AddLocalOffset` (`/Game/Props/Blueprints/Interactables/Battery/BP_BatteryLightComponent.DefaultSceneRoot` _array_element) (* (/ (* _returnvalue (`self.BalleryLightOffset`)) 2.0) -1.0) false false)))))