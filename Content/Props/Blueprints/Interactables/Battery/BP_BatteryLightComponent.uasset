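; Battery light prop that shows a lit or unlit state for the battery interactables.
; TurnOn and TurnOff toggle the PointLight's visibility and swap BatteryMesh between lit and unlit dev materials, with an emission fade Timeline noted but not built.
; GetBatteryLightRef returns a success flag and a self reference for other Blueprints.
; The event graph and construction script are empty, so state changes only through calls to these functions.
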(event `self.ReceiveBeginPlay`)

(fn `GetBatteryLightRef`
  (returns (Success :type Boolean) (Ref :type "/Game/Props/Blueprints/Interactables/Battery/BP_BatteryLightComponent Object Reference"))
  (return true self))

(fn `TurnOff`
  (`SceneComponent.SetVisibility` (`self.PointLight`) false false)
  ;[1 1 1] Make Timeline to adjust material emission brightness over time
  (`PrimitiveComponent.SetMaterial` (`self.BatteryMesh`) 0 "/Game/Props/Textures/Materials/Battery/MAT_Dev_UnlitLight.MAT_Dev_UnlitLight"))

(fn `TurnOn`
  (`SceneComponent.SetVisibility` (`self.PointLight`) true false)
  ;[1 1 1] Make Timeline to adjust material emission brightness over time
  (`PrimitiveComponent.SetMaterial` (`self.BatteryMesh`) 0 "/Game/Props/Textures/Materials/Battery/MAT_Dev_LitLight.MAT_Dev_LitLight"))

(fn `UserConstructionScript`)