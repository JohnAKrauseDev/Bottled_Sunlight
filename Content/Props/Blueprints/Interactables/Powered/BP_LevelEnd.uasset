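; BP_LevelEnd is an interactable prop that ends the current level by opening the level set in LevelToLoad.
; PrimaryInteract accepts only a BP_Sunkiss_Character and, when NeedsPower is set, also requires IsPowered before calling LevelEnd.
; It returns whether the interaction succeeded, and LevelEnd opens the level by object reference with a debug print.
; The event graph holds only disabled default events.
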(fn `LevelEnd`
  (`GameplayStatics.OpenLevelBySoftObjectPtr` (`self.LevelToLoad`))
  (`KismetSystemLibrary.PrintString` "End LEvel"))

(fn `PrimaryInteract`
  (params (Instegator :type "Actor Object Reference"))
  (returns (Success :type Boolean))
  (cast `/Game/Player/Blueprints/BP_Sunkiss_Character` Instegator
    (:`then`
      (if (`self.NeedsPower`)
        (if (`self.IsPowered`)
          (`self.LevelEnd`)
          (return true)
          (else
            (return false)))
        (else
          (`self.LevelEnd`)
          (return true))))
    (:`CastFailed`
      (return false))))

(fn `UserConstructionScript`
  (`parent.UserConstructionScript`))