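; BP_PoweredLights is a light prop that switches on and off with its powered state.
; StartPowered and EndPowered extend the parent's functions, swapping the LightMesh material between lit and unlit dev materials and toggling the RectLight's visibility.
; The construction script sets the RectLight's intensity from FloorGlowIntensity.
; The event graph only forwards BeginPlay to the parent, alongside an unreachable delayed visibility-toggle chain and an empty stray event.
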(event `self.ReceiveBeginPlay`
  (`parent.ReceiveBeginPlay`))

(event `wtf`)

(fn `EndPowered`
  (`parent.EndPowered`)
  (`PrimitiveComponent.SetMaterial` (`self.LightMesh`) 0 "/Game/Props/Textures/Materials/Battery/MAT_Dev_UnlitLight.MAT_Dev_UnlitLight")
  (`SceneComponent.SetVisibility` (`self.RectLight`) false false))

(fn `StartPowered`
  (`parent.StartPowered`)
  (`PrimitiveComponent.SetMaterial` (`self.LightMesh`) 0 "/Game/Props/Textures/Materials/Battery/MAT_Dev_LitLight.MAT_Dev_LitLight")
  (`SceneComponent.SetVisibility` (`self.RectLight`) true false))

(fn `UserConstructionScript`
  (`parent.UserConstructionScript`)
  (`LightComponent.SetIntensity` (`self.RectLight`) (`self.FloorGlowIntensity`)))