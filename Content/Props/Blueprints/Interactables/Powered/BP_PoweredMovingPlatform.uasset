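; Powered moving platform prop, a prototype that travels in a straight line between start and end offsets from its placed location once powered.
; The construction script computes world endpoints and scales the mesh; StartPowered starts a fast looping timer that steps the root by Speed.
; A dot product detects overshooting an endpoint, then reverses direction, or pauses at the end without Loop.
; EndPowered only calls its parent, and notes suggest replacing this with splines.
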(event `self.ReceiveBeginPlay`
  ;[1 1 1] Temporary for testing pourposes
  (`parent.ReceiveBeginPlay`))

(event `MovePlatform`
  (bind _defaultsceneroot (`self.DefaultSceneRoot`))
  (bind _returnvalue (`SceneComponent.K2_GetComponentLocation` (`self.DefaultSceneRoot`)))
  (bind _returnvalue_2 (>= (`KismetMathLibrary.Dot_VectorVector` (`KismetMathLibrary.GetDirectionUnitVector` _returnvalue (`self.WorldStart`)) (`KismetMathLibrary.GetDirectionUnitVector` _returnvalue (`self.WorldEnd`))) 0.0))
  ;[1 0 0.03977] Bad, dont keep if prototype fun, use splines instead
  ;;[1 1 1] Called by timer
  (if (`self.IsMovingForward`)
    (`SceneComponent.K2_SetWorldLocation` _defaultsceneroot (+ (`SceneComponent.K2_GetComponentLocation` (`self.DefaultSceneRoot`)) (* (`KismetMathLibrary.GetDirectionUnitVector` (`self.Start`) (`self.End`)) (`self.Speed`))) false false)
    ;;[1 1 1] If start and end are not oposite directions, turn around
    (if _returnvalue_2
      (if (`self.Loop`)
        (set `self.IsMovingForward` false)
        (else
          (`KismetSystemLibrary.K2_PauseTimerHandle` (struct)))))
    (else
      (`SceneComponent.K2_SetWorldLocation` _defaultsceneroot (+ (`SceneComponent.K2_GetComponentLocation` (`self.DefaultSceneRoot`)) (* (`KismetMathLibrary.GetDirectionUnitVector` (`self.End`) (`self.Start`)) (`self.Speed`))) false false)
      (if _returnvalue_2
        (set `self.IsMovingForward` true)))))

(fn `EndPowered`
  (`parent.EndPowered`))

(fn `StartPowered`
  ;[1 0.07239 0.06244] Bad, dont keep if prototype fun
  (`parent.StartPowered`)
  (bind _returnvalue (`KismetSystemLibrary.K2_SetTimer` null "movePlatform" 0.001 true))
  (set `self.MovingTimer` _returnvalue))

(fn `UserConstructionScript`
  (`parent.UserConstructionScript`)
  (set `self.WorldStart` (+ (`self.Start`) (`SceneComponent.K2_GetComponentLocation` (`self.DefaultSceneRoot`))))
  (set `self.WorldEnd` (+ (`self.End`) (`SceneComponent.K2_GetComponentLocation` (`self.DefaultSceneRoot`))))
  (`SceneComponent.SetWorldScale3D` (`self.PlatformMesh`) (`self.PlatformDimensions`)))