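; Base Blueprint for interactable props that run on power, with an option for child variants that need none, such as the level end.
; The construction script adds the actor to the DependantRefs list of each assigned power source, skipping duplicates.
; StartPowered and EndPowered toggle the IsPowered flag.
; BeginPlay calls StartPowered immediately when NeedsPower is off.
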(event `self.ReceiveBeginPlay`
  ;[1 1 1] For powered children that i want to be able to have no powere neded variants, namely level end
  (`parent.ReceiveBeginPlay`)
  (if (not (`self.NeedsPower`))
    (`self.StartPowered`)))

(fn `EndPowered`
  (set `self.IsPowered` false))

(fn `StartPowered`
  (set `self.IsPowered` true))

(fn `UserConstructionScript`
  (`parent.UserConstructionScript`)
  (for _array_element (`self.PowerSources`)
    (bind _dependantrefs (`/Game/Props/Blueprints/Interactables/Battery/BP_Battery.DependantRefs` _array_element))
    (if (not (`KismetArrayLibrary.Array_Contains` _dependantrefs self))
      (`KismetArrayLibrary.Array_Add` _dependantrefs self))))