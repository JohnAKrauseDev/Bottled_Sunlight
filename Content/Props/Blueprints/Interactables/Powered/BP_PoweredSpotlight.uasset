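; BP_PoweredSpotlight is a powered prop whose spotlight turns on and off with its power state.
; The construction script applies intensity, color temperature and attenuation radius to the SpotLight component.
; StartPowered and EndPowered call their parent versions, then show or hide the light.
; The event graph holds only disabled default events.
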(fn `EndPowered`
  (`parent.EndPowered`)
  (`SceneComponent.SetVisibility` (`self.SpotLight`) false false))

(fn `StartPowered`
  (`parent.StartPowered`)
  (`SceneComponent.SetVisibility` (`self.SpotLight`) true false))

(fn `UserConstructionScript`
  (bind _spotlight (`self.SpotLight`))
  (`parent.UserConstructionScript`)
  (`LightComponent.SetIntensity` _spotlight (`self.New Intensity`))
  (`LightComponent.SetTemperature` _spotlight (`self.New Temperature`))
  (`LocalLightComponent.SetAttenuationRadius` _spotlight (`self.New Radius`)))