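; Tutorial text prop that shows a world-space text message while the player character is nearby.
; The construction script sizes the trigger sphere from Radius and formats four editable line variables into the TextRender's text.
; BeginPlay sets initial visibility from a StartVisibly flag.
; Sphere overlap events show the text when a BP_Sunkiss_Character enters and hide it on exit.
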(event `self.ReceiveBeginPlay`
  (`SceneComponent.SetVisibility` (`self.TextRender`) (`self.StartVisibly`) false))

(event `self.Sphere.OnComponentBeginOverlap`
  (params (OverlappedComponent :type "PrimitiveComponent Object Reference") (OtherActor :type "Actor Object Reference") (OtherComp :type "PrimitiveComponent Object Reference") (OtherBodyIndex :type Integer) (bFromSweep :type Boolean) (SweepResult :type "HitResult Structure (by ref)"))
  (cast `/Game/Player/Blueprints/BP_Sunkiss_Character` OtherActor)
  (`SceneComponent.SetVisibility` (`self.TextRender`) true false))

(event `self.Sphere.OnComponentEndOverlap`
  (params (OverlappedComponent :type "PrimitiveComponent Object Reference") (OtherActor :type "Actor Object Reference") (OtherComp :type "PrimitiveComponent Object Reference") (OtherBodyIndex :type Integer))
  (cast `/Game/Player/Blueprints/BP_Sunkiss_Character` OtherActor)
  (`SceneComponent.SetVisibility` (`self.TextRender`) false false))

(fn `UserConstructionScript`
  (`SphereComponent.SetSphereRadius` (`self.Sphere`) (`self.Radius`) true)
  (`TextRenderComponent.K2_SetText` (`self.TextRender`) (`|FormatText` "{l1} \n{l2} \n{l3} \n{l4}" (`self.Line1`) (`self.Line2`) (`self.Line3`) (`self.Line4`))))